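; A practice pawn that moves and looks from input axes and prints debug messages.
; Forward and right axes offset the actor along its own vectors without sweep or delta-time scaling.
; LookUp drives controller yaw and LookRight drives pitch, the reverse of their names.
; Tick feeds ShowTimeSet, which accumulates time and prints each new whole second, while BeginPlay, W and EnterInput print fixed strings.
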(event EventBeginPlay
  (Development|PrintString "BeginPlay"))

(event EventTick
  (params (DeltaSeconds :type Float%20%28single-precision%29))
  (CallFunction|ShowTimeSet DeltaSeconds))

(event Input|ActionEvents|InputActionEnterInput
  (params (Key :type Key%20Structure :default "None"))
  (:Pressed
    (Development|PrintString "Hello")))

(event Input|AxisEvents|InputAxisLookRight
  (params (AxisValue :type Float%20%28single-precision%29))
  (Pawn|Input|AddControllerPitchInput AxisValue))

(event Input|AxisEvents|InputAxisLookUp
  (params (AxisValue :type Float%20%28single-precision%29))
  (Pawn|Input|AddControllerYawInput AxisValue))

(event Input|AxisEvents|InputAxisfoward
  (params (AxisValue :type Float%20%28single-precision%29))
  ;[1 1 1] 앞 뒤 움직임
  (Transformation|AddActorWorldOffset (* (Transformation|GetActorForwardVector) (* AxisValue 1e+01))))

(event Input|AxisEvents|InputAxisMoveRight
  (params (AxisValue :type Float%20%28single-precision%29))
  (Transformation|AddActorWorldOffset (* (Transformation|GetActorRightVector) (* AxisValue 1e+01))))

(event Input|KeyboardEvents|W
  (params (Key :type Key%20Structure :default "None"))
  (:Pressed
    (Development|PrintString "w key")))

(fn ConstructionScript)

(fn ShowTimeSet
  (params (DeltaSecond :type Float%20%28single-precision%29))
  (bind _output_get (Variables|Default|Settotal%20delta%20seconds (+ DeltaSecond (Variables|Default|Gettotal%20delta%20seconds))))
  (if (not (== (Variables|Default|GetBefore%20Int) (Math|Float|Floor _output_get)))
    (Development|PrintString (Utilities|String|Append "Delta Seconds-" (Utilities|String|ToString(Integer) (Math|Float|Floor _output_get))))
    (Variables|Default|SetBefore%20Int (Math|Float|Floor _output_get))))
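; Actor Blueprint that moves itself back and forth along X through its DefaultSceneRoot.
; Tick adds a relative X offset scaled by Speed and delta time, with the Ismovelight flag choosing between the forward step and the alternate, apparently reversed, step.
; The flag clears above X 100 and sets again at or below that same threshold, so motion settles into oscillation around that point rather than sweeping between two bounds.
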(event EventBeginPlay)

(event Collision|EventActorBeginOverlap
  (params (OtherActor :type Actor%20Object%20Reference)))

(event EventTick
  (params (DeltaSeconds :type Float%20%28single-precision%29))
  (bind _speed (Variables|Default|Getspeed))
  (bind _defaultsceneroot (Variables|Default|GetDefaultSceneRoot))
  (bind _returnvalue (* DeltaSeconds _speed))
  (if (Variables|Default|GetIsmovelight)
    (Transformation|AddRelativeLocation _defaultsceneroot (Math|Vector|MakeVector _returnvalue 0.0 0.0) false false)
    (if (> (.x (Variables|/Script/Engine.SceneComponent|GetRelativeLocation _defaultsceneroot)) 1e+02)
      (Variables|Default|SetIsmovelight false))
    (else
      (bind _result (Math|Float|NegateFloat _returnvalue)
        (:%20%20
          (Transformation|AddRelativeLocation _defaultsceneroot (Math|Vector|MakeVector _result 0.0 0.0) false false)
          (if (<= (.x (Variables|/Script/Engine.SceneComponent|GetRelativeLocation _defaultsceneroot)) 1e+02)
            (Variables|Default|SetIsmovelight true)))))))

(fn ConstructionScript)